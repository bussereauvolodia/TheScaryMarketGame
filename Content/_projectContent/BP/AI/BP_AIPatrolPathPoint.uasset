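; BP_AIPatrolPathPoint is an AI patrol point that reports whether it is accessible and whether it sits inside a nav modifier volume.
; It caches the first-person player on BeginPlay and picks one of three accessibility flags from the player's completed task count, defaulting to the first without a valid task list.
; Helper functions check its linked nav modifiers, testing the cylinder's location against each one's bounding box.
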(event EventBeginPlay
  (bind _asbp_first_person_character (Utilities|Casting|CastToBP_FirstPersonCharacter (Game|GetPlayerCharacter 0)))
  (Variables|Default|SetPlayer _asbp_first_person_character))

(event Collision|EventActorBeginOverlap
  (params (OtherActor :type Actor%20Object%20Reference)))

(event EventTick
  (params (DeltaSeconds :type Float%20%28single-precision%29)))

(fn ConstructionScript)

(fn FIsActorinNavModifierVolume
  (for _array_element (Variables|Default|GetNavMeshModifiers)
    (Utilities|IsValid _array_element
      (:Is%20Valid
        (if (Class|KismetMathLibrary|IsPointinBoxwithTransform (Transformation|GetWorldLocation (Variables|Default|GetCylinder)) (Transformation|GetActorTransform _array_element) (.BoxExtent (Collision|GetActorBounds _array_element false false)))
          (return true)))))
  (return false))

(fn FIsActorLinktoNavModifierVolume
  (for _array_element (Variables|Default|GetNavMeshModifiers)
    (Utilities|IsValid _array_element
      (:Is%20Valid
        (return "true"))))
  (return "false"))

(fn FIsActorAccessible
  (bind _player (Variables|Default|GetPlayer))
  (bind _tasklist (Variables|/Game/_projectContent/BP/BP_FirstPersonCharacter.BP_FirstPersonCharacter_C|GetTaskList _player))
  (Utilities|IsValid _tasklist
    (:Is%20Valid
      (switch int (Default|GetNumberOfTaskCompleted _tasklist)
        (:0
          (return (Variables|Default|GetAccessibleOntask1)))
        (:1
          (return (Variables|Default|GetAccessibleOnTask2)))
        (:2
          (return (Variables|Default|GetAccessibleOnTask3)))))
    (:Is%20Not%20Valid
      (return (Variables|Default|GetAccessibleOntask1)))))