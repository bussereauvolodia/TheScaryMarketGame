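; BP_MallZone is a safe-zone volume that tracks whether the player is inside its box and informs the AI and audio.
; Each zone broadcasts ZoneUpdate on overlap changes and a first-tick check; entering also clears the AI's NeedToRadar key.
; The zone flagged as main listens to its SafeZones list, combines their states, then updates the IsPlayerInSafeZone blackboard key and notifies BP_AudioManager.
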(event OnComponentBeginOverlap(Box)
  (params (OverlappedComponent :type Primitive%20Component%20Object%20Reference) (OtherActor :type Actor%20Object%20Reference) (OtherComp :type Primitive%20Component%20Object%20Reference) (OtherBodyIndex :type Integer) (bFromSweep :type Boolean) (SweepResult :type Hit%20Result%20Structure%20%28by%20ref%29))
  (if (== OtherActor (Variables|Default|GetPlayer))
    (Variables|Default|SetIsInSafeZone true)
    (AI|Components|Blackboard|ClearValue (AI|GetBlackboard (Variables|Default|GetAIController)) (Utilities|Name|MakeLiteralName "NeedToRadar"))
    (Default|CallZoneUpdate true)))

(event OnComponentEndOverlap(Box)
  (params (OverlappedComponent :type Primitive%20Component%20Object%20Reference) (OtherActor :type Actor%20Object%20Reference) (OtherComp :type Primitive%20Component%20Object%20Reference) (OtherBodyIndex :type Integer))
  (if (== OtherActor (Variables|Default|GetPlayer))
    (Variables|Default|SetIsInSafeZone false)
    (Default|CallZoneUpdate false)))

(event Custom|CE_UpdateBlackboard
  (if (Variables|Default|GetIsTheMainSafeZone)
    (AI|Components|Blackboard|SetValueasBool (AI|GetBlackboard (Variables|Default|GetAIController)) (Utilities|Name|MakeLiteralName "IsPlayerInSafeZone") (CallFunction|FIsPlayerinSafeZones))))

(event Custom|ZoneUpdated
  (params (IsInZone :type Boolean))
  (if IsInZone
    (Variables|Default|SetIsInSafeZoneS true)
    (else
      (Variables|Default|SetIsInSafeZoneS (CallFunction|FIsPlayerinSafeZones))))
  (CallFunction|CEUpdateBlackboard)
  (Default|ChangedZone (Variables|Default|GetAudioManager) (Variables|Default|GetIsInSafeZoneS))
  (Development|PrintString (Utilities|String|ToString(Boolean) (Variables|Default|GetIsInSafeZoneS))))

(event EventBeginPlay
  (bind _returnvalue (Actor|GetActorOfClass "/Game/_projectContent/BP/AI/AI_Controller.AI_Controller_C"))
  (Variables|Default|SetAIController _returnvalue)
  (bind _returnvalue_2 (Actor|GetActorOfClass "/Game/_projectContent/BP/Sound/BP_AudioManager.BP_AudioManager_C"))
  (Variables|Default|SetAudioManager _returnvalue_2)
  (if (Variables|Default|GetIsTheMainSafeZone)
    (for _array_element (Variables|Default|GetSafeZones)
      (EventDispatchers|BindEventtoZoneUpdate _array_element (EventDispatchers|CreateEvent :!event Custom|ZoneUpdated)))))

(event EventTick
  (params (DeltaSeconds :type Float%20%28single-precision%29))
  (Utilities|FlowControl|DoOnce false
    (:Completed
      (bind _returnvalue (Actor|GetActorOfClass "/Game/_projectContent/BP/BP_FirstPersonCharacter.BP_FirstPersonCharacter_C"))
      (bind _output_get (Variables|Default|SetPlayer _returnvalue))
      (bind _output_get_2 (Variables|Default|SetIsInSafeZone (Collision|IsOverlappingActor (Variables|Default|GetBox) _output_get :!class /Script/Engine.PrimitiveComponent)))
      (Default|CallZoneUpdate _output_get_2))))

(fn ConstructionScript)

(fn FIsPlayerinSafeZones
  (if (Variables|Default|GetIsInSafeZone)
    (return (Variables|Default|GetIsInSafeZone))
    (else
      (for _array_element (Variables|Default|GetSafeZones)
        (Utilities|IsValid _array_element
          (:Is%20Valid
            (if (Variables|BP_MallZone_C|GetIsInSafeZone _array_element)
              (return true)))))
      (return false))))