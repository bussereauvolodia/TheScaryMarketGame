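; BP_Monster is the AI monster character that hunts the player, driven by blackboard keys on its AI controller.
; A timeline expands a radar zone with a sound moving toward the player; overlapping a player whose badge is active rings it and sets TargetActor.
; Other events handle sound effects, timeline-smoothed rotation, walk speed, and resetting the monster to its spawn transform while clearing attack and QTE states.
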(event OnComponentBeginOverlap(RadarZone)
  (params (OverlappedComponent :type Primitive%20Component%20Object%20Reference) (OtherActor :type Actor%20Object%20Reference) (OtherComp :type Primitive%20Component%20Object%20Reference) (OtherBodyIndex :type Integer) (bFromSweep :type Boolean) (SweepResult :type Hit%20Result%20Structure%20%28by%20ref%29))
  (Utilities|IsValid (AI|Components|Blackboard|GetValueasObject (AI|GetBlackboard (Variables|Default|GetAs%20AI%20Controller)) (Utilities|Name|MakeLiteralName "TargetActor"))
    (:Is%20Not%20Valid
      (bind _asbp_first_person_character (Utilities|Casting|CastToBP_FirstPersonCharacter OtherActor))
      (bind _badgeblueprint (Variables|/Game/_projectContent/BP/BP_FirstPersonCharacter.BP_FirstPersonCharacter_C|GetBadgeBlueprint _asbp_first_person_character)
        (:then
          (if (Variables|/Game/_projectContent/BP/BP_Badge.BP_Badge_C|GetIsActive _badgeblueprint)
            (bind _as_ai_controller (Variables|Default|GetAs%20AI%20Controller)
              (:then
                (AI|Components|Blackboard|SetValueasObject (AI|GetBlackboard _as_ai_controller) (Utilities|Name|MakeLiteralName "TargetActor") _asbp_first_person_character)
                (Default|RingingBadge _badgeblueprint)
                (CallFunction|CEResetRadarZone))
              (:else))))
        (:else)))))

(event Custom|CE_RadarZone
  (params (DistanceDetection :type Float%20%28double-precision%29) (TimeToScan :type Float%20%28double-precision%29))
  (bind _bp_sfxcomponent (Variables|Default|GetBP_SFXComponent))
  (bind _radarzone (Variables|Default|GetRadarZone))
  (bind _audio_component (Default|FGetAudioComponentfromName _bp_sfxcomponent "Monster_ElectricalRelease"))
  (bind _returnvalue (Transformation|GetWorldLocation _audio_component))
  (Rendering|SetVisibility (Variables|Default|GetRadarZone) true false)
  (Components|Timeline|SetPlayRate (Variables|Default|GetT_RadarScale) (/ 1.0 TimeToScan))
  (Default|PlaySFX (Variables|Default|GetBP_SFXComponent) "Monster_ElectricalRelease" (Transformation|GetActorLocation) 1.0 self)
  (bind _scanningzonescaling (Timeline|T_RadarScale PlayFromStart)
    (:Update
      ;[1 1 1] Le son du radar follow l'expansion de la zone
      (Transformation|SetRelativeScale3D _radarzone (Math|Vector|Lerp(Vector) "0.100000,0.100000,0.100000" (Math|Conversions|ToVector(Float) DistanceDetection) _scanningzonescaling))
      (Utilities|IsValid _audio_component
        (:Is%20Valid
          (Transformation|SetWorldLocation _audio_component (+ _returnvalue (* (Math|Vector|GetUnitDirection(Vector) _returnvalue (Transformation|GetWorldLocation (Variables|/Script/Engine.Character|GetCapsuleComponent (Variables|Default|GetAs%20BP%20First%20Person%20Character)))) (Variables|/Script/Engine.SceneComponent|GetRelativeScale3D _radarzone))) false false))))
    (:Finished
      (CallFunction|CEResetRadarZone))))

(event Custom|CE_ResetMonster
  (bind _spawntransform (Variables|Default|GetSpawnTransform))
  (bind _as_ai_controller (Variables|Default|GetAs%20AI%20Controller))
  (bind _blackboard (Variables|/Script/AIModule.AIController|GetBlackboard _as_ai_controller))
  (Transformation|SetActorLocationAndRotation (.location _spawntransform) (.rotation _spawntransform) false true)
  (AI|Components|Blackboard|ClearValue _blackboard (Utilities|Name|MakeLiteralName "IsAttacking"))
  (AI|Components|Blackboard|ClearValue _blackboard (Utilities|Name|MakeLiteralName "IsInQTE"))
  (Rendering|SetActorHiddenInGame false)
  (CallFunction|CEStopChaseSound)
  (Default|StopSFXfromName (Variables|Default|GetBP_SFXComponent) "Monster_Screamer"))

(event Custom|CE_SoundEvent
  (params (SFXName :type String) (Multiplier :type Float%20%28double-precision%29))
  (Default|PlaySFX (Variables|Default|GetBP_SFXComponent) SFXName (Transformation|GetActorLocation) Multiplier self))

(event Custom|CE_RotateTowardLocation
  (params (Target%20World%20Location :type Vector%20%28by%20ref%29) (RotationSpeed :type Float%20%28double-precision%29))
  (bind _capsulecomponent (Variables|Collision|GetCapsuleComponent))
  (bind _returnvalue (Transformation|GetWorldRotation _capsulecomponent))
  (Components|Timeline|SetPlayRate (Variables|Default|GetT_RotateToward) (/ 1.0 RotationSpeed))
  (bind _rotate (Timeline|T_RotateToward Play)
    (:Update
      (Transformation|SetWorldRotation (Variables|Collision|GetCapsuleComponent) (Math|Rotator|MakeRotator (.roll _returnvalue) (.pitch _returnvalue) (Math|Float|Lerp (.yaw _returnvalue) (.yaw (Math|Rotator|FindLookatRotation (Transformation|GetWorldLocation _capsulecomponent) Target%20World%20Location)) _rotate)) false false)
      (Pawn|SetControlRotation (Variables|Default|GetAs%20AI%20Controller) (Math|Rotator|MakeRotator (.roll _returnvalue) (.pitch _returnvalue) (Math|Float|Lerp (.yaw _returnvalue) (.yaw (Math|Rotator|FindLookatRotation (Transformation|GetWorldLocation _capsulecomponent) Target%20World%20Location)) _rotate))))))

(event Custom|CE_ResetRotation
  (params (Rotation%20Speed :type Float%20%28double-precision%29))
  (Components|Timeline|SetPlayRate (Variables|Default|GetT_ResetRotation) (/ 1.0 Rotation%20Speed))
  (bind _rotate (Timeline|T_ResetRotation PlayFromStart)
    (:Update
      (Transformation|SetWorldRotation (Variables|Collision|GetCapsuleComponent) (Math|Rotator|MakeRotator 0.0 0.0 (Math|Float|Lerp (.yaw (Transformation|GetWorldRotation (Variables|Collision|GetCapsuleComponent))) (.yaw (Pawn|GetControlRotation (Variables|Default|GetAs%20AI%20Controller) :!class /Script/Engine.Controller)) _rotate)) false false))))

(event Custom|CE_ResetRadarZone
  (bind _radarzone (Variables|Default|GetRadarZone))
  (bind _as_ai_controller (Variables|Default|GetAs%20AI%20Controller))
  (bind _returnvalue (AI|GetBlackboard _as_ai_controller))
  (if (Audio|Components|Audio|IsPlaying (Variables|Default|GetT_RadarScale))
    (Audio|Components|Audio|Stop (Variables|Default|GetT_RadarScale)))
  (Rendering|SetVisibility _radarzone false false)
  (Transformation|SetRelativeScale3D _radarzone "0, 0, 0")
  (AI|Components|Blackboard|SetValueasBool _returnvalue (Utilities|Name|MakeLiteralName "IsScanning") false)
  (AI|Components|Blackboard|SetValueasBool _returnvalue (Utilities|Name|MakeLiteralName "NeedToRadar") false)
  (Default|StopSFXfromName (Variables|Default|GetBP_SFXComponent) "Monster_ElectricalRelease"))

(event Custom|CE_StopChaseSound
  (if (Audio|Components|Audio|IsPlaying (Variables|Default|GetAudio))
    (Audio|Components|Audio|Stop (Variables|Default|GetAudio))
    (AI|Components|Blackboard|SetValueasBool (Variables|/Script/AIModule.AIController|GetBlackboard (Variables|Default|GetAs%20AI%20Controller)) (Utilities|Name|MakeLiteralName "IsAlreadyPlayingChaseSound") false)))

(event EventBeginPlay
  (bind _asai_controller (Utilities|Casting|CastToAI_Controller (AI|GetAIController self)))
  (Variables|Default|SetAs%20AI%20Controller _asai_controller)
  (bind _ashud_in_game (Utilities|Casting|CastToHUD_InGame (HUD|GetHUD (Game|GetPlayerController 0))))
  (Variables|Default|SetAs%20HUD%20In%20Game _ashud_in_game)
  (Variables|Default|SetSpawnTransform (Transformation|GetActorTransform))
  (bind _asbp_first_person_character (Utilities|Casting|CastToBP_FirstPersonCharacter (Game|GetPlayerCharacter 0)))
  (Variables|Default|SetAs%20BP%20First%20Person%20Character _asbp_first_person_character))

(event Collision|EventActorBeginOverlap
  (params (OtherActor :type Actor%20Object%20Reference)))

(event EventTick
  (params (DeltaSeconds :type Float%20%28single-precision%29)))

(fn ConstructionScript)

(fn FUpdateWalkSpeed
  (params (NewWalkSpeed :type Float%20%28double-precision%29))
  (Variables|/Script/Engine.CharacterMovementComponent|SetMaxWalkSpeed (Variables|Character|GetCharacterMovement) NewWalkSpeed)
  (return))