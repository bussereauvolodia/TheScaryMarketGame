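; Interactable sound-emitting object that can report itself to the BP_Monster AI.
; Interact plays its SFX and locks interaction until the sound's duration ends, then fires FinishedSound unless already re-enabled or destroyed.
; FSoundToAI writes it to the monster's blackboard; the ultrasound variant also sets a trigger flag and clears TargetActor.
; Turning it off stops the sound, then reboots normal objects after a delay or permanently breaks ultrasound ones, clearing the flag.
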(event Custom|CE_TurnOfDestroy
  (Default|StopSFX (Variables|Default|GetBP_SFXComponent))
  (if (Variables|Default|GetIsUltraSound)
    (Components|StaticMesh|SetStaticMesh (Variables|Default|GetCube) (Variables|Default|GetBrokenMesh))
    (Rendering|Material|SetMaterial (Variables|Default|GetCube) 0 (Variables|Default|GetBrokenMaterial))
    (AI|Components|Blackboard|SetValueasBool (AI|GetBlackboard (Variables|Default|GetAIController)) (Utilities|Name|MakeLiteralName "IsTriggerByUltraSound") false)
    (Variables|Default|SetIsDestroyed true)
    (else
      (Utilities|FlowControl|Delay (Variables|Default|GetTimeBeforeReboot))
      (Variables|Default|SetCanInterract true))))

(event Custom|FinishedSound)

(event EventBeginPlay
  (bind _returnvalue (Actor|GetActorOfClass "/Game/_projectContent/BP/AI/BP_Monster.BP_Monster_C"))
  (Variables|Default|SetAIController (AI|GetAIController _returnvalue)))

(event Collision|EventActorBeginOverlap
  (params (OtherActor :type Actor%20Object%20Reference)))

(event EventTick
  (params (DeltaSeconds :type Float%20%28single-precision%29)))

(event EventInteract
  (params (Character :type BP%20First%20Person%20Character%20Object%20Reference))
  (if (Variables|Default|GetCanInterract)
    (bind _soundduration (Default|PlaySFX (Variables|Default|GetBP_SFXComponent) (Variables|PlaySFXValues|GetSFXName) (Transformation|GetActorLocation) 1.0 self))
    (Variables|Default|SetCanInterract false)
    ;[1 1 1] Si le son a fini d'être joué sans être éteint alors on peut ré intéragir
    (Utilities|FlowControl|Delay _soundduration)
    (if (Variables|Default|GetIsUltraSound)
      (if (not (Variables|Default|GetIsDestroyed))
        (if (not (Variables|Default|GetCanInterract)) :!label _label
          (Variables|Default|SetCanInterract true)
          (CallFunction|FinishedSound)))
      (else
        (goto _label)))))

(event EventIsPointed
  (params (IsPointed :type Boolean)))

(fn ConstructionScript)

(fn FSoundtoAI
  (bind _aicontroller (Variables|Default|GetAIController))
  (bind _returnvalue (AI|GetBlackboard _aicontroller))
  (AI|Components|Blackboard|SetValueasObject (AI|GetBlackboard (Variables|Default|GetAIController)) (Utilities|Name|MakeLiteralName "SoundObject") self)
  (if (Variables|Default|GetIsUltraSound)
    (AI|Components|Blackboard|SetValueasBool _returnvalue (Utilities|Name|MakeLiteralName "IsTriggerByUltraSound") true)
    (AI|Components|Blackboard|ClearValue _returnvalue (Utilities|Name|MakeLiteralName "TargetActor"))))

(fn CanInteract
  (return (not (Variables|Default|GetCanInterract))))