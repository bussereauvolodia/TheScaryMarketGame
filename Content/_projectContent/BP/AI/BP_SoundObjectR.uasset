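; Interactable sound-emitting object that plays a configurable SFX, optionally perceptible to AI.
; Interact plays it through BPSFXComponent and blocks re-interaction for the delay that call returns.
; CE_TurnOfDestroy stops the sound, then either re-enables interaction after a reboot delay or, for ultrasound objects, swaps to a broken mesh.
; The ultrasound branch also clears IsTriggerByUltraSound on the BP_Monster AI blackboard, using the controller cached at BeginPlay.
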(event Custom|CE_TurnOfDestroy
  (Default|StopSFX (Variables|Default|GetBP_SFXComponent))
  (if (Variables|Default|GetIsUltraSound)
    (Components|StaticMesh|SetStaticMesh (Variables|Default|GetCube) (Variables|Default|GetBrokenMesh))
    (AI|Components|Blackboard|SetValueasBool (AI|GetBlackboard (Variables|Default|GetAIController)) (Utilities|Name|MakeLiteralName "IsTriggerByUltraSound") false)
    (else
      (Utilities|FlowControl|Delay (Variables|Default|GetTimeBeforeReboot))
      (Variables|Default|SetCanInterract true))))

(event EventBeginPlay
  (bind _returnvalue (Actor|GetActorOfClass "/Game/_projectContent/BP/AI/BP_Monster.BP_Monster_C"))
  (Variables|Default|SetAIController (AI|GetAIController _returnvalue)))

(event Collision|EventActorBeginOverlap
  (params (OtherActor :type Actor%20Object%20Reference)))

(event EventTick
  (params (DeltaSeconds :type Float%20%28single-precision%29)))

(event EventInteract
  (params (Character :type BP%20First%20Person%20Character%20Object%20Reference))
  (if (Variables|Default|GetCanInterract)
    (bind _soundduration (Default|PlaySFX (Variables|Default|GetBP_SFXComponent) (Variables|PlaySFXValues|GetSFXName) (Transformation|GetActorLocation) (Variables|PlaySFXValues|GetIntensity) (Variables|PlaySFXValues|GetIs%20IASensible) (Variables|PlaySFXValues|GetSFXTag) self (Variables|PlaySFXValues|GetMax%20Range) (Variables|PlaySFXValues|GetConcurrency%20Settings) (Variables|PlaySFXValues|GetAuto%20Destroy)))
    (Variables|Default|SetCanInterract false)
    (Utilities|FlowControl|Delay _soundduration)
    ;[1 1 1] Si le son a fini d'être joué sans être éteint alors on peut ré intéragir
    (if (not (Variables|Default|GetCanInterract))
      (Variables|Default|SetCanInterract true))))

(fn ConstructionScript)