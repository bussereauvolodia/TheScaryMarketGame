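; BP_SoundObject_ChildT is a sound object child Blueprint that adds visual feedback to its parent's interaction by swapping the Cube's material.
; It caches the Cube's original material at BeginPlay, applies OnMaterial on Interact when CanInterract is true, then calls the parent's Interact.
; The FinishedSound event restores the cached material.
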(event EventBeginPlay
  (Variables|Default|SetBaseMat (Rendering|Material|GetMaterial (Variables|Default|GetCube) 0))
  (|CallParentFunction))

(event Collision|EventActorBeginOverlap
  (params (OtherActor :type Actor%20Object%20Reference))
  (|CallParentFunction OtherActor))

(event EventTick
  (params (DeltaSeconds :type Float%20%28single-precision%29))
  (|CallParentFunction DeltaSeconds) ; This node is disabled and will not be called.\nDrag off pins to build functionality.
)

(event EventInteract
  (params (Character :type BP%20First%20Person%20Character%20Object%20Reference))
  (Utilities|FlowControl|Sequence
    (:then_0
      (if (Variables|Default|GetCanInterract)
        (Rendering|Material|SetMaterial (Variables|Default|GetCube) 0 (Variables|Default|GetOnMaterial))
        (Development|PrintString "ChangedMesh")))
    (:then_1
      (|CallParentFunction 0))))

(event EventFinishedSound
  (Rendering|Material|SetMaterial (Variables|Default|GetCube) 0 (Variables|Default|GetBaseMat)))

(fn ConstructionScript
  (|CallParentFunction))