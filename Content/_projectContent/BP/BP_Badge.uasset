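; BP_Badge is a badge with a mesh and a widget screen that can be temporarily deactivated.
; On BeginPlay it disables shadow casting on both parts and caches the screen's WD_Badge widget.
; DeactivateBadge, when the badge is active, sets the widget inactive, hides the screen after a turn-off delay, then restores both after a turn-on delay.
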(event Custom|Deactivate%20Badge
  (if (Variables|Default|GetIsActive)
    (Default|SetActive (Variables|Default|GetBadgeWidget) false)
    (Utilities|FlowControl|Delay (Variables|Default|GetTurnOffCooldown))
    (Variables|Default|SetIsActive false)
    (Development|SetHiddeninGame (Variables|Default|GetScreen) true false)
    (Utilities|FlowControl|Delay (Variables|Default|GetTurnOnCooldown))
    (Variables|Default|SetIsActive true)
    (Default|SetActive (Variables|Default|GetBadgeWidget) true)
    (Development|SetHiddeninGame (Variables|Default|GetScreen) false false)))

(event EventBeginPlay
  (Rendering|SetCastShadow (Variables|Default|GetBadge) false)
  (Rendering|SetCastShadow (Variables|Default|GetScreen) false)
  (bind _aswd_badge (Utilities|Casting|CastToWD_Badge (UserInterface|GetWidget (Variables|Default|GetScreen))))
  (Variables|Default|SetBadgeWidget _aswd_badge)
  (Utilities|Casting|CastToBP_FirstPersonCharacter (Game|GetPlayerCharacter 0)))

(fn ConstructionScript)