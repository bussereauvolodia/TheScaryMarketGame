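; BP_CinematicManager starts a Level Sequence when the first-person player enters its trigger box, and sets the player's IsHidding flag.
; On BeginPlay it caches the player character and finds the BP_SO_ChildSeqSensible actor used as an alarm clock.
; RingClock manually launches the clock's sound, while StopSequence clears the flag and stops the sequence.
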(event OnComponentBeginOverlap(TriggerBox)
  (params (OverlappedComponent :type Primitive%20Component%20Object%20Reference) (OtherActor :type Actor%20Object%20Reference) (OtherComp :type Primitive%20Component%20Object%20Reference) (OtherBodyIndex :type Integer) (bFromSweep :type Boolean) (SweepResult :type Hit%20Result%20Structure%20%28by%20ref%29))
  (bind _player (Variables|Default|GetPlayer))
  (bind _levelsequence (Variables|Default|GetLevelSequence))
  (if (== _player OtherActor)
    (Variables|/Game/_projectContent/BP/BP_FirstPersonCharacter.BP_FirstPersonCharacter_C|SetIsHidding _player true)
    (Utilities|IsValid _levelsequence
      (:Is%20Valid
        (Sequencer|Player|Play (Variables|/Script/LevelSequence.LevelSequenceActor|GetSequencePlayer _levelsequence) :!class /Script/MovieScene.MovieSceneSequencePlayer)))))

(event Custom|RingClock
  (Default|LaunchSoundManually (Variables|Default|GetAlarmClock)))

(event Custom|StopSequence
  (Variables|/Game/_projectContent/BP/BP_FirstPersonCharacter.BP_FirstPersonCharacter_C|SetIsHidding (Variables|Default|GetPlayer) false)
  (Sequencer|Player|Stop (Variables|/Script/LevelSequence.LevelSequenceActor|GetSequencePlayer (Variables|Default|GetLevelSequence)) :!class /Script/MovieScene.MovieSceneSequencePlayer))

(event EventBeginPlay
  (bind _asbp_first_person_character (Utilities|Casting|CastToBP_FirstPersonCharacter (Game|GetPlayerCharacter 0)))
  (Variables|Default|SetPlayer _asbp_first_person_character)
  (bind _returnvalue (Actor|GetActorOfClass "/Game/_projectContent/BP/BP_SO_ChildSeqSensible.BP_SO_ChildSeqSensible_C"))
  (Variables|Default|SetAlarmClock _returnvalue))

(fn ConstructionScript)