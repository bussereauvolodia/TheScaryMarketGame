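; BP_DoorTriggerZone is a trigger volume that reports whether the player is inside it, named for use with doors.
; Its Box overlap events filter for player character 0 and set IsInZone on enter and exit.
; Both paths print a French debug message, then call the TriggerChange dispatcher with the new state, leaving any reaction to listeners.
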(event OnComponentBeginOverlap(Box)
  (params (OverlappedComponent :type Primitive%20Component%20Object%20Reference) (OtherActor :type Actor%20Object%20Reference) (OtherComp :type Primitive%20Component%20Object%20Reference) (OtherBodyIndex :type Integer) (bFromSweep :type Boolean) (SweepResult :type Hit%20Result%20Structure%20%28by%20ref%29))
  (if (== OtherActor (Game|GetPlayerCharacter 0))
    (Variables|Default|SetIsInZone true)
    (Development|PrintString "DANS LA ZOOONE")
    (Default|CallTriggerChange (Variables|Default|GetIsInZone))))

(event OnComponentEndOverlap(Box)
  (params (OverlappedComponent :type Primitive%20Component%20Object%20Reference) (OtherActor :type Actor%20Object%20Reference) (OtherComp :type Primitive%20Component%20Object%20Reference) (OtherBodyIndex :type Integer))
  (if (== OtherActor (Game|GetPlayerCharacter 0))
    (Variables|Default|SetIsInZone false)
    (Development|PrintString "AP DANS LA ZOOONE")
    (Default|CallTriggerChange (Variables|Default|GetIsInZone))))

(fn ConstructionScript)