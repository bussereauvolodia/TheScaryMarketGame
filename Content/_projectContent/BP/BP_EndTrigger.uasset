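; BP_EndTrigger is a trigger volume that ends the game by launching the credits when the player walks into it.
; On BeginPlay it caches the player's HUD_InGame.
; When the player character overlaps its Box, it calls LaunchCredits on that HUD and, if FreezePlayer is set, disables the character's movement.
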(event OnComponentBeginOverlap(Box)
  (params (OverlappedComponent :type Primitive%20Component%20Object%20Reference) (OtherActor :type Actor%20Object%20Reference) (OtherComp :type Primitive%20Component%20Object%20Reference) (OtherBodyIndex :type Integer) (bFromSweep :type Boolean) (SweepResult :type Hit%20Result%20Structure%20%28by%20ref%29))
  (bind _returnvalue (Game|GetPlayerCharacter 0))
  (bind _hud (Variables|Default|GetHUD))
  (if (== _returnvalue OtherActor)
    (Utilities|IsValid _hud
      (:Is%20Valid
        (Default|LaunchCredits _hud)
        (if (Variables|Default|GetFreezePlayer)
          (Pawn|Components|CharacterMovement|DisableMovement (Variables|/Script/Engine.Character|GetCharacterMovement _returnvalue)))))))

(event EventBeginPlay
  (bind _ashud_in_game (Utilities|Casting|CastToHUD_InGame (HUD|GetHUD (Game|GetPlayerController 0))))
  (Variables|Default|SetHUD _ashud_in_game))

(fn ConstructionScript)