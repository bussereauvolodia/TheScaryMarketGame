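; BP_FinalDoor is a double sliding door that opens once the level's task list reports enough finished tasks.
; On BeginPlay it caches both panel positions and binds to the task completion event of BP_TaskList.
; When the count reaches NbTasks, a speed-scaled timeline lerps the panels to the StandRight and StandLeft positions, with a door SFX.
; CloseDoor only plays the sound and clears IsOpen; it does not move the panels.
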(event Custom|OnTaskCompletion
  (params (NbFinishedTask :type Integer))
  (if (>= NbFinishedTask (Variables|Default|GetNbTasks))
    (CallFunction|OpenDoor)))

(event Custom|OpenDoor
  (CallFunction|SFXDoor)
  (Variables|Default|SetIsOpen true)
  (bind _lerpvalue (Timeline|OpenTimeline Play)
    (:Update
      (CallFunction|UpdateDoorsPos _lerpvalue))))

(event Custom|CloseDoor
  (CallFunction|SFXDoor)
  (Variables|Default|SetIsOpen false))

(event EventBeginPlay
  (Variables|Default|SetRightDoorLocation (Variables|/Script/Engine.SceneComponent|GetRelativeLocation (Variables|Default|GetRightDoor)))
  (Variables|Default|SetLeftDoorLocation (Variables|/Script/Engine.SceneComponent|GetRelativeLocation (Variables|Default|GetLeftDoor)))
  (Components|Timeline|SetPlayRate (Variables|Default|GetOpenTimeline) (Variables|Default|GetDoorSpeed))
  (bind _returnvalue (Actor|GetActorOfClass "/Game/_projectContent/BP/BP_TaskList.BP_TaskList_C"))
  (bind _output_get (Variables|Default|SetTaskList _returnvalue))
  (EventDispatchers|BindEventtoOnTaskCompletion _output_get (EventDispatchers|CreateEvent :!event Custom|OnTaskCompletion)))

(fn ConstructionScript)

(fn UpdateDoorsPos
  (params (Alpha :type Float%20%28double-precision%29))
  (Transformation|SetRelativeLocation (Variables|Default|GetRightDoor) (Math|Vector|Lerp(Vector) (Variables|Default|GetRightDoorLocation) (Variables|/Script/Engine.SceneComponent|GetRelativeLocation (Variables|Default|GetStandRight)) Alpha) false false)
  (Transformation|SetRelativeLocation (Variables|Default|GetLeftDoor) (Math|Vector|Lerp(Vector) (Variables|Default|GetLeftDoorLocation) (Variables|/Script/Engine.SceneComponent|GetRelativeLocation (Variables|Default|GetStandLeft)) Alpha) false false))

(fn SFXDoor
  (Default|PlaySFX (Variables|Default|GetBP_SFXComponent) "GlassDoorOpenClose" (Transformation|GetActorLocation) 1.0 self))