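; BP_FlickeringLamp2 is a lamp actor whose spot light flickers on and off at irregular intervals.
; On Tick, a Delay of FlickFreq plus a random offset within plus or minus RandomValue gates a FlipFlop.
; The FlipFlop alternates the SpotLight intensity between zero and DefaultIntensity and records the state in IsOn.
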(event EventTick
  (params (DeltaSeconds :type Float%20%28single-precision%29))
  (bind _randomvalue (Variables|Default|GetRandomValue))
  (bind _spotlight (Variables|Default|GetSpotLight))
  (Utilities|FlowControl|Delay (+ (Variables|Default|GetFlickFreq) (Math|Random|RandomFloatinRange (* _randomvalue -1.0) _randomvalue)))
  (Utilities|FlowControl|FlipFlop
    (:A
      (Rendering|Components|Light|SetIntensity _spotlight 0.0)
      (Variables|Default|SetIsOn false))
    (:B
      (Rendering|Components|Light|SetIntensity _spotlight (Variables|Default|GetDefaultIntensity))
      (Variables|Default|SetIsOn true))))

(fn ConstructionScript)