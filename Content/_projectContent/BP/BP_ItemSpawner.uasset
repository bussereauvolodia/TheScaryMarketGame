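; BP_ItemSpawner spawns named items at random positions for a given task.
; On BeginPlay it converts each ItemSpawnables entry's placed position actors into stored locations and destroys those actors.
; SpawnItemsOfTask selects entries matching the task name, then spawns up to each entry's count of BP_ItemTest actors, setting their item name.
; Each chosen location is removed from the entry's list as it is used.
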(event Custom|SpawnItemsOfTask
  (params (TaskName :type String))
  (bind _itemspawnable (CallFunction|GetSpawnableItems TaskName))
  (for _array_element _itemspawnable
    (CallFunction|SpawnItems _array_element)))

(event EventBeginPlay
  (bind _itemspawnables (Variables|Default|GetItemSpawnables))
  (for (_array_element _array_index) _itemspawnables
    (for _array_element_2 (.possiblepositionsbp _array_element)
      (Utilities|Array|Add (.positionslist (Utilities|Array|Get(acopy) _itemspawnables _array_index)) (Transformation|GetActorLocation _array_element_2))
      (Actor|DestroyActor _array_element_2))))

(fn ConstructionScript)

(fn GetSpawnableItems
  (params (TaskName :type String))
  (bind _itemspawnlist (LocalVariables|GetItemSpawnList))
  (for _array_element (Variables|Default|GetItemSpawnables)
    (if (Utilities|Enum|Equal(Enum) TaskName (.SpawningTaskName (Utilities|Struct|BreakST_ItemSpawnInfos _array_element)))
      (Utilities|Array|Add _itemspawnlist _array_element)))
  (return _itemspawnlist))

(fn SpawnItems
  (params (ItemSpawnable :type ST%20Item%20Spawn%20Infos%20Structure))
  (for _index (range 0 (- (.count ItemSpawnable) 1))
    (if (> (Utilities|Array|Length (.positionslist ItemSpawnable)) 0)
      (bind _output_get (LocalVariables|SetSelectedPos (.OutItem (Utilities|Array|Random (.positionslist ItemSpawnable)))))
      (bind _returnvalue (Game|SpawnActorfromClass "/Game/_projectContent/BP/BP_ItemTest.BP_ItemTest_C" (Math|Transform|MakeTransform _output_get "0, 0, 0" "1.000000,1.000000,1.000000") "Undefined" "MultiplyWithRoot" 0 0))
      (Default|SetItem _returnvalue (.itemname ItemSpawnable))
      (Utilities|Array|RemoveItem (.positionslist ItemSpawnable) _output_get))))