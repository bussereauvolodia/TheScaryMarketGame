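; Test item pickup actor, shown as a Paper2D sprite that turns every Tick to face the player like a billboard.
; GetItem looks up ItemName in DT_ItemInformations, printing empty or missing names, and BeginPlay applies that row's sprite.
; PickUpItem plays an explosion SFX flagged as AI-sensible through BPSFXComponent, destroys the actor and returns the item info to the caller.
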(event EventBeginPlay
  (bind _iteminfo (CallFunction|GetItem))
  (Rendering|Components|Sprite|SetSprite (Variables|Default|GetPaperSprite) (.sprite _iteminfo)))

(event EventTick
  (params (DeltaSeconds :type Float%20%28single-precision%29))
  (Transformation|SetActorRotation (Math|Rotator|FindLookatRotation (Transformation|GetActorLocation) (Transformation|GetActorLocation (Game|GetPlayerCharacter 0)))))

(fn ConstructionScript)

(fn GetItem
  (bind _itemname (Variables|Default|GetItemName))
  (if (not (Utilities|Array|IsEmpty _itemname))
    (bind _returnvalue (Utilities|GetDataTableRow "/Game/_projectContent/DataTables/DT_ItemInformations.DT_ItemInformations" (Utilities|String|StringToName _itemname))
      (:then
        (return _returnvalue true))
      (:RowNotFound
        (Development|PrintString (Utilities|String|Append "The Item \"" (Variables|Default|GetItemName) "\" Does not exist"))
        (return "" false)))
    (else
      (Development|PrintString "ItemName is Empty"))))

(fn PickUpItem
  (bind (_iteminfo _hasitem) (CallFunction|GetItem))
  (if _hasitem
    (Default|PlaySFX (Variables|Default|GetBP_SFXComponent) "Explosion" (Transformation|GetActorLocation) 0.5 true "Item")
    (Actor|DestroyActor)
    (return _iteminfo)))