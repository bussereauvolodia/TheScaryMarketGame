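; BP_LockedDoor is an interactable double door that opens only for a character with an active badge and a specific gameplay item selected.
; A dot product sign picks the swing direction, and a timeline rotates both leaves in opposite yaw.
; After a cooldown, a second timeline closes them using the left leaf's current yaw sign, then clears IsOpen.
; With no item selected, it prints the item enum.
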(event EventInteract
  (params (Character :type BP%20First%20Person%20Character%20Object%20Reference))
  (bind (_hasitem _gp_item) (Default|GetSelectedItem Character))
  (bind _leftdoor (Variables|Default|GetLeftDoor))
  (bind _badgeblueprint (Variables|/Game/_projectContent/BP/BP_FirstPersonCharacter.BP_FirstPersonCharacter_C|GetBadgeBlueprint Character))
  (Utilities|IsValid _badgeblueprint
    (:Is%20Valid
      (if _hasitem
        (if (and (Variables|/Game/_projectContent/BP/BP_Badge.BP_Badge_C|GetIsActive _badgeblueprint) (Utilities|Enum|Equal(Enum) (.gameplayitem _gp_item) "NewEnumerator4"))
          (if (not (Variables|Default|GetIsOpen))
            (Variables|Default|SetRotSign (Math|Float|Sign(Float) (|DotofVectors_2 Character)))
            (Variables|Default|SetIsOpen true)
            (bind _rotationvalue (Timeline|OpenTimeline PlayFromStart)
              (:Update
                (Transformation|SetRelativeRotation (Variables|Default|GetRightDoor) (Math|Rotator|MakeRotator 0.0 0.0 (* _rotationvalue (Variables|Default|GetRotSign))) false false)
                (Transformation|SetRelativeRotation (Variables|Default|GetLeftDoor) (Math|Rotator|MakeRotator 0.0 0.0 (* (* _rotationvalue (Variables|Default|GetRotSign)) -1.0)) false false))
              (:Finished
                (Utilities|FlowControl|Delay (Variables|Default|GetClosingCooldown))
                (bind _rotationvalue_2 (Timeline|CloseTimeline PlayFromStart)
                  (:Update
                    (Transformation|SetRelativeRotation _leftdoor (Math|Rotator|MakeRotator 0.0 0.0 (* _rotationvalue_2 (Math|Float|Sign(Float) (.yaw (Variables|/Script/Engine.SceneComponent|GetRelativeRotation _leftdoor))))) false false)
                    (Transformation|SetRelativeRotation (Variables|Default|GetRightDoor) (Math|Rotator|MakeRotator 0.0 0.0 (* (* _rotationvalue_2 (Math|Float|Sign(Float) (.yaw (Variables|/Script/Engine.SceneComponent|GetRelativeRotation _leftdoor)))) -1.0)) false false))
                  (:Finished
                    (Variables|Default|SetIsOpen false)))))))
        (else
          (Development|PrintString (Utilities|String|EnumtoString (.gameplayitem _gp_item))))))))

(fn ConstructionScript)