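; BP_Locker is an interactable hiding locker that lets the player evade the monster.
; Toggling hide aligns the player, animates the door, blends the view to the locker, and removes the player from AI perception and collision.
; If the monster has a target or investigates nearby, the locker writes itself to the AI blackboard and starts a HUD QTE.
; Success clears those keys, while failure exposes and damages the player.
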(event OnComponentBeginOverlap(Box)
  (params (OverlappedComponent :type Primitive%20Component%20Object%20Reference) (OtherActor :type Actor%20Object%20Reference) (OtherComp :type Primitive%20Component%20Object%20Reference) (OtherBodyIndex :type Integer) (bFromSweep :type Boolean) (SweepResult :type Hit%20Result%20Structure%20%28by%20ref%29))
  ;[1 1 1] Hide and UnHide in Locker
  (bind _asbp_first_person_character (Utilities|Casting|CastToBP_FirstPersonCharacter OtherActor))
  (bind _output_get (Variables|Default|SetAs%20BP%20First%20Person%20Character _asbp_first_person_character))
  (Utilities|FlowControl|Gate true) ; enters at Open
)

(event OnComponentEndOverlap(Box)
  (params (OverlappedComponent :type Primitive%20Component%20Object%20Reference) (OtherActor :type Actor%20Object%20Reference) (OtherComp :type Primitive%20Component%20Object%20Reference) (OtherBodyIndex :type Integer))
  ;[1 1 1] Hide and UnHide in Locker
  (Utilities|Casting|CastToBP_FirstPersonCharacter OtherActor)
  (Utilities|FlowControl|Gate true) ; enters at Close
)

(event Custom|CE_ToggleHide
  (bind _returnvalue (Game|GetPlayerController 0))
  (bind _arrow (Variables|Default|GetArrow))
  (bind _as_bp_first_person_character (Variables|Default|GetAs%20BP%20First%20Person%20Character))
  (bind _blend_time (Variables|Default|GetBlend%20Time))
  (bind _as_bp_first_person_character_2 (Variables|Default|GetAs%20BP%20First%20Person%20Character))
  (bind _returnvalue_2 (Transformation|GetActorLocation _as_bp_first_person_character))
  (bind _returnvalue_3 (Transformation|GetWorldLocation _arrow))
  (bind _rootcomponent (Variables|/Script/Engine.Actor|GetRootComponent _as_bp_first_person_character))
  (bind _returnvalue_4 (Math|Vector|MakeVector (.x _returnvalue_3) (.y _returnvalue_3) (.z _returnvalue_2)))
  ;[1 1 1] Toggle Hidding
  (if (Variables|Default|GetCanInterractWithLocker)
    (Variables|Default|SetCanInterractWithLocker false)
    (if (Variables|Default|GetIsHidding)
      (Variables|Default|SetIsHidding false)
      (|GoOutLocker
        (:execute
          (Game|Player|SetViewTargetwithBlend _returnvalue (Variables|Default|GetAs%20BP%20First%20Person%20Character) _blend_time "VTBlend_Linear" 0.0 false)
          (Utilities|FlowControl|Delay (Variables|Default|GetBlend%20Time))
          (Default|SelectGameplayItem (Variables|Default|GetAs%20BP%20First%20Person%20Character) (Variables|Default|GetSelectedItem))
          (CallFunction|FPlayerAppeartoAI)
          (Variables|/Game/_projectContent/BP/BP_FirstPersonCharacter.BP_FirstPersonCharacter_C|SetIsHidding (Variables|Default|GetAs%20BP%20First%20Person%20Character) (Variables|Default|GetIsHidding) :!label _label)))
      (else
        (bind _output_get (Variables|Default|SetIsHidding true))
        (Variables|/Game/_projectContent/BP/BP_FirstPersonCharacter.BP_FirstPersonCharacter_C|SetIsHidding _as_bp_first_person_character_2 _output_get)
        (Variables|Default|SetSelectedItem (Variables|/Game/_projectContent/BP/BP_FirstPersonCharacter.BP_FirstPersonCharacter_C|GetSelectedIndex _as_bp_first_person_character_2))
        (Default|SelectGameplayItem _as_bp_first_person_character_2)
        (CallFunction|CEUpdateLockerLocation)
        (Utilities|FlowControl|Sequence
          (:then_0
            (if (Utilities|Operators|NotEqual(!=) (Transformation|GetWorldLocation _rootcomponent) _returnvalue_4 3.0)
              (Components|MoveComponentTo _rootcomponent _returnvalue_4 "0, 0, 0" true true 1.0 true))
            (|GoInLocker
              (:execute
                (Game|Player|SetViewTargetwithBlend _returnvalue self _blend_time "VTBlend_Linear" 0.0 false)
                (CallFunction|FPlayerDissappeartoAI)
                (goto _label))))
          (:then_1
            (CallFunction|CELookatDoor)))))))

(event Custom|CE_LookAtDoor
  (bind _returnvalue (Transformation|GetActorLocation))
  (bind _returnvalue_2 (Game|GetPlayerController 0))
  (bind _as_bp_first_person_character (Variables|Default|GetAs%20BP%20First%20Person%20Character))
  (bind _heightlookatlocker (Variables|Default|GetHeightLookAtLocker))
  (bind _returnvalue_3 (Transformation|GetActorLocation _as_bp_first_person_character))
  (bind _returnvalue_4 (Math|Rotator|FindLookatRotation _returnvalue_3 (Math|Vector|MakeVector (.x _returnvalue) (.y _returnvalue) _heightlookatlocker)))
  ;[1 1 1] Handle the player camera rotation toward the locker
  (if (Utilities|Operators|NotEqual(!=) (Pawn|GetControlRotation (Variables|Default|GetAs%20BP%20First%20Person%20Character) :!class /Script/Engine.Pawn) _returnvalue_4 3.0)
    (Input|DisableInput (Variables|Default|GetAs%20BP%20First%20Person%20Character) (Game|GetPlayerController 0))
    (Timeline|T_LookAtLocker PlayFromStart
      (:Update
        (Pawn|SetControlRotation _returnvalue_2 (Math|Interpolation|RInterpTo (Pawn|GetControlRotation (Variables|Default|GetAs%20BP%20First%20Person%20Character) :!class /Script/Engine.Pawn) _returnvalue_4 (Utilities|Time|GetWorldDeltaSeconds) 4.0)))
      (:Finished
        (Input|EnableInput (Variables|Default|GetAs%20BP%20First%20Person%20Character) _returnvalue_2)))))

(event Custom|CE_UpdateLockerLocation
  (bind _as_ai_controller (Variables|Default|GetAs%20AI%20Controller))
  (bind _returnvalue (AI|GetBlackboard _as_ai_controller))
  ;[1 1 1] Si le joueur est pris en chasse lorsqu'il rentre dans le casier
  (if (or (Utilities|IsValid (AI|Components|Blackboard|GetValueasObject (AI|GetBlackboard (Variables|Default|GetAs%20AI%20Controller)) (Utilities|Name|MakeLiteralName "TargetActor"))) (<= (Math|Vector|Distance(Vector) (AI|Components|Blackboard|GetValueasVector (AI|GetBlackboard (Variables|Default|GetAs%20AI%20Controller)) (Utilities|Name|MakeLiteralName "InvestigationLocation")) (Transformation|GetActorLocation)) (Variables|Default|GetDistanceMonsterNearLockerToActivateQTE)))
    (AI|Components|Blackboard|SetValueasVector _returnvalue (Utilities|Name|MakeLiteralName "LastLockerLocation") (Transformation|GetWorldLocation (Variables|Default|GetArrow)))
    (AI|Components|Blackboard|SetValueasObject _returnvalue (Utilities|Name|MakeLiteralName "Locker") self)
    (Variables|Default|SetDoQTE true)))

(event Custom|CE_ClearLockerLocation
  (AI|Components|Blackboard|ClearValue (AI|GetBlackboard (Variables|Default|GetAs%20AI%20Controller)) (Utilities|Name|MakeLiteralName "LastLockerLocation"))
  (AI|Components|Blackboard|ClearValue (AI|GetBlackboard (Variables|Default|GetAs%20AI%20Controller)) (Utilities|Name|MakeLiteralName "InvestigationLocation"))
  (Variables|Default|SetDoQTE false)
  (AI|Components|Blackboard|ClearValue (AI|GetBlackboard (Variables|Default|GetAs%20AI%20Controller)) (Utilities|Name|MakeLiteralName "IsInQTE")))

(event Custom|ChaseValueChanged
  (params (IsChased :type Boolean))
  (Variables|Default|SetIs%20Chased IsChased))

(event EventQTEFInished
  (params (Success :type Boolean))
  (if Success
    (CallFunction|CEClearLockerLocation)
    (else
      (Development|PrintString "Looser")
      (Variables|Default|SetCanInterractWithLocker true)
      (CallFunction|CEToggleHide)
      (CallFunction|CEClearLockerLocation)
      (Variables|Default|SetDoQTE false)
      (CallFunction|FPlayerAppeartoAI)
      (bind _output_get (Variables|Default|SetIsHidding false))
      (Variables|/Game/_projectContent/BP/BP_FirstPersonCharacter.BP_FirstPersonCharacter_C|SetIsHidding (Variables|Default|GetAs%20BP%20First%20Person%20Character) _output_get)
      (Default|FDamage (Variables|Default|GetAs%20BP%20First%20Person%20Character)))))

(event EventBeginPlay
  (bind _returnvalue (Actor|GetActorOfClass "/Game/_projectContent/BP/AI/BP_Monster.BP_Monster_C"))
  (bind _output_get (Variables|Default|SetMonster _returnvalue))
  (bind _asai_controller (Utilities|Casting|CastToAI_Controller (AI|GetAIController _output_get)))
  (bind _output_get_2 (Variables|Default|SetAs%20AI%20Controller _asai_controller))
  (EventDispatchers|BindEventtoEDonChaseValueChange _output_get_2 (EventDispatchers|CreateEvent :!event Custom|ChaseValueChanged))
  (bind _ashud_in_game (Utilities|Casting|CastToHUD_InGame (HUD|GetHUD (Game|GetPlayerController 0))))
  (Variables|Default|SetAs%20HUD%20In%20Game _ashud_in_game))

(event EventIsPointed
  (params (IsPointed :type Boolean))
  (bind _locker (Variables|Default|GetLocker))
  (Rendering|SetRenderCustomDepth _locker IsPointed)
  (Rendering|SetCustomDepthStencilValue _locker (Math|Integer|SelectInt 1 0 IsPointed)))

(event EventInteract
  (params (Character :type BP%20First%20Person%20Character%20Object%20Reference))
  ;[1 1 1] Hide and UnHide in Locker
  (Utilities|FlowControl|Gate true :!label _label
    (:Exit
      (Default|CESetPostProcessSettings (stale OnComponentBeginOverlap(Box) _output_get) (Variables|Default|GetPostProcess))
      (CallFunction|CEToggleHide)
      (Utilities|FlowControl|Delay 1.0)
      (goto _label Open))))

(fn ConstructionScript
  (Rendering|Debug|DrawDebugSphere (Transformation|GetWorldLocation (Variables|Default|GetCamera)) (Variables|Default|GetDistanceMonsterNearLockerToActivateQTE) 12 "(R=1.000000,G=1.000000,B=1.000000,A=1.000000)" 0.5 1.0))

(fn FPlayerAppeartoAI
  (bind _as_bp_first_person_character (Variables|Default|GetAs%20BP%20First%20Person%20Character))
  (Rendering|SetActorHiddenInGame _as_bp_first_person_character false)
  (Collision|SetActorEnableCollision _as_bp_first_person_character true)
  (Class|AIPerceptionStimuliSourceComponent|RegisterwithPerceptionSystem (Variables|/Game/_projectContent/BP/BP_FirstPersonCharacter.BP_FirstPersonCharacter_C|GetAIPerceptionStimuliSource _as_bp_first_person_character))
  (return))

(fn FPlayerDissappeartoAI
  (bind _as_bp_first_person_character (Variables|Default|GetAs%20BP%20First%20Person%20Character))
  (Rendering|SetActorHiddenInGame _as_bp_first_person_character true)
  (Collision|SetActorEnableCollision _as_bp_first_person_character false)
  (Class|AIPerceptionStimuliSourceComponent|UnregisterfromPerceptionSystem (Variables|/Game/_projectContent/BP/BP_FirstPersonCharacter.BP_FirstPersonCharacter_C|GetAIPerceptionStimuliSource _as_bp_first_person_character))
  (return))

(fn CanInteract
  (return false))