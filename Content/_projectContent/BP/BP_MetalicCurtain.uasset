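; Metallic curtain actor that rises while CanMoveUp is set and drops back after a delay when released, until it reaches full height.
; Tick moves it by constant-speed interpolation between OpenHeight and the Z captured at BeginPlay, using Gate and DoOnce nodes to sequence delay and sounds.
; Reaching the top locks it open and destroys its NavVolumeModifier.
; BPSFXComponent plays the movement sounds, scaled by CurtainNoise.
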(event Custom|CE_PlaySound
  (params (SFXName :type String))
  (Default|PlaySFX (Variables|Default|GetBP_SFXComponent) SFXName (Transformation|GetActorLocation) (Variables|Default|GetCurtainNoise) self))

(event Custom|CE_StopSound
  (Default|StopSFX (Variables|Default|GetBP_SFXComponent)))

(event EventBeginPlay
  ;[1 1 1] Comme le pivot est au mileu je le multiplie par deux pour avoir la position du rideau fermé
  (Variables|Default|SetCloseHeight (.z (Transformation|GetActorLocation))))

(event Collision|EventActorBeginOverlap
  (params (OtherActor :type Actor%20Object%20Reference)))

(event EventTick
  (params (DeltaSeconds :type Float%20%28single-precision%29))
  (bind _returnvalue (Transformation|GetActorLocation))
  (bind _returnvalue_2 (Transformation|GetActorLocation))
  (bind _returnvalue_3 (Transformation|GetActorLocation))
  (bind _returnvalue_4 (Transformation|GetActorLocation))
  (bind _navvolumemodifier (Variables|Default|GetNavVolumeModifier))
  (if (not (Variables|Default|GetisFullyOpened))
    (if (Variables|Default|GetCanMoveUp)
      (Utilities|FlowControl|Sequence
        (:then_0
          (Transformation|SetActorLocation (Math|Vector|MakeVector (.x _returnvalue) (.y _returnvalue) (Math|Interpolation|FInterptoConstant (.z _returnvalue) (Variables|Default|GetOpenHeight) DeltaSeconds (Variables|Default|GetOpeningSpeed))) false false)
          (Utilities|FlowControl|Sequence
            (:then_0
              (if (Utilities|Operators|EqualEqual (Math|Vector|MakeVector (.x _returnvalue_3) (.y _returnvalue_3) (.z _returnvalue_3)) (Math|Vector|MakeVector (.x _returnvalue_3) (.y _returnvalue_3) (Variables|Default|GetOpenHeight)) 1.0)
                (Variables|Default|SetisFullyOpened true)
                (CallFunction|CEStopSound)
                (CallFunction|CEPlaySound "MetalicCurtainOpen")
                (Utilities|IsValid _navvolumemodifier
                  (:Is%20Valid
                    (Actor|DestroyActor _navvolumemodifier)))))
            (:then_1
              (Utilities|FlowControl|DoOnce false :!label _label
                (:Completed
                  (Utilities|FlowControl|Sequence
                    (:then_0
                      (CallFunction|CEPlaySound "MetalicCurtainOpening"))
                    (:then_1
                      (goto _label_5 Reset))))))))
        (:then_1
          (goto _label_4 Close))
        (:then_2
          (goto _label_3 Reset))
        (:then_3
          (goto _label_2 Reset)))
      (else
        (Utilities|FlowControl|Sequence
          (:then_0
            (if (Utilities|Operators|EqualEqual (Math|Vector|MakeVector (.x _returnvalue_2) (.y _returnvalue_2) (.z _returnvalue_2)) (Math|Vector|MakeVector (.x _returnvalue_2) (.y _returnvalue_2) (Variables|Default|GetCloseHeight)) 1.0)
              (Utilities|FlowControl|DoOnce true :!label _label_2
                (:Completed
                  (CallFunction|CEStopSound)
                  (CallFunction|CEPlaySound "MetalicCurtainClose")))
              (else
                (Utilities|FlowControl|Sequence
                  (:then_0
                    (Utilities|FlowControl|DoOnce false :!label _label_3
                      (:Completed
                        (CallFunction|CEStopSound)
                        (Utilities|FlowControl|Delay (Variables|Default|GetTimeBeforeClosingAgain))
                        (goto _label_4 Open))))
                  (:then_1
                    (Utilities|FlowControl|Gate true :!label _label_4
                      (:Exit
                        (Utilities|FlowControl|Sequence
                          (:then_0
                            (Transformation|SetActorLocation (Math|Vector|MakeVector (.x _returnvalue_4) (.y _returnvalue_4) (Math|Interpolation|FInterptoConstant (.z _returnvalue_4) (Variables|Default|GetCloseHeight) DeltaSeconds (Variables|Default|GetClosingSpeed))) false false))
                          (:then_1
                            (Utilities|FlowControl|DoOnce false :!label _label_5
                              (:Completed
                                (CallFunction|CEPlaySound "MetalicCurtainOpening"))))))))))))
          (:then_1
            (goto _label Reset)))))))

(fn ConstructionScript)