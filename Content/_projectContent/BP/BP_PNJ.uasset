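; BP_PNJ is an interactable NPC that gives the player a task and rewards its completion.
; It turns on yaw every tick to face the player character.
; On Interact, a character with a task list first collects the NPC's task, and later interactions attempt completion against that character's inventory and grant the returned gameplay item on success.
; Dialogue is currently placeholder debug prints.
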(event EventTick
  (params (DeltaSeconds :type Float%20%28single-precision%29))
  (bind _returnvalue (Transformation|GetActorRotation))
  (Transformation|SetActorRotation (Math|Rotator|MakeRotator (.roll _returnvalue) (.pitch _returnvalue) (.yaw (Math|Rotator|FindLookatRotation (Transformation|GetActorLocation) (Transformation|GetActorLocation (Game|GetPlayerCharacter 0)))))))

(event EventInteract
  (params (Character :type BP%20First%20Person%20Character%20Object%20Reference))
  (bind _tasklist (Variables|/Game/_projectContent/BP/BP_FirstPersonCharacter.BP_FirstPersonCharacter_C|GetTaskList Character))
  (Variables|Default|SetCharacter Character)
  (Utilities|IsValid _tasklist
    (:Is%20Valid
      (if (Variables|Default|GetHasCollectedTask)
        (if (not (Default|IsTaskComplete (Variables|Default|GetBP_TaskHandler)))
          (Development|PrintString "Dialogue completing tasj")
          (bind (_iscomplete _gameplay_item) (Default|CompleteTask (Variables|Default|GetBP_TaskHandler) (Variables|/Game/_projectContent/BP/BP_FirstPersonCharacter.BP_FirstPersonCharacter_C|GetInventory (Variables|Default|GetCharacter))))
          (if _iscomplete
            (Default|CollectGameplayItem (Variables|Default|GetCharacter) (Utilities|Struct|MakeST_GameplayItem _gameplay_item 0))))
        (else
          (Development|PrintString "Dialogue collect task")
          (Default|CollectTask _tasklist (Variables|Default|GetBP_TaskHandler))
          (Variables|Default|SetHasCollectedTask true))))
    (:Is%20Not%20Valid
      (Development|PrintString "Dialogue need collect list"))))

(fn ConstructionScript)