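; BP_PNJCurtain is a curtain linked to an NPC (PNJ) that opens once the preceding NPC's task is complete.
; On BeginPlay it stores its root X scale as the closed value and binds to the task-changed event on the BPTaskHandler of PNJ.BeforePNJ.
; When that task reports complete, a timeline lerps the root's X scale from closed to open, with Y and Z held at one.
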(event Custom|TaskChanged
  (if (Default|IsTaskComplete (Variables|/Game/_projectContent/BP/BP_PNJ.BP_PNJ_C|GetBP_TaskHandler (Variables|/Game/_projectContent/BP/BP_PNJ.BP_PNJ_C|GetBeforePNJ (Variables|Default|GetPNJ))))
    (bind _lerp (Timeline|Timeline Play)
      (:Update
        (Transformation|SetRelativeScale3D (Variables|Default|GetDefaultSceneRoot) (Math|Vector|MakeVector (Math|Float|Lerp (Variables|Default|GetClosedScale) (Variables|Default|GetOpenScale) _lerp) 1.0 1.0))))))

(event EventBeginPlay
  (EventDispatchers|BindEventtoTaskChanged (Variables|/Game/_projectContent/BP/BP_PNJ.BP_PNJ_C|GetBP_TaskHandler (Variables|/Game/_projectContent/BP/BP_PNJ.BP_PNJ_C|GetBeforePNJ (Variables|Default|GetPNJ))) (EventDispatchers|CreateEvent :!event Custom|TaskChanged))
  (Variables|Default|SetClosedScale (.x (Variables|/Script/Engine.SceneComponent|GetRelativeScale3D (Variables|Default|GetDefaultSceneRoot)))))

(fn ConstructionScript)