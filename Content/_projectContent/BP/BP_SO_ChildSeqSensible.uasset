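; BP_SO_ChildSeqSensible is a child Blueprint of an interactable sound-playing object, linked to a cinematic sequence.
; LaunchSoundManually stores the CinematicManager passed to it, then calls Interact to trigger the object.
; Its CETurnOfDestroy override runs the parent logic, then tells that stored manager to stop the sequence.
; BeginPlay, overlap, Tick and construction add no logic of their own.
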(event Custom|LaunchSoundManually
  (params (CinematicManager :type BP%20Cinematic%20Manager%20Object%20Reference))
  (Variables|Default|SetCinematic%20Manager CinematicManager)
  (CallFunction|Interact))

(event EventBeginPlay
  (|CallParentFunction) ; This node is disabled and will not be called.\nDrag off pins to build functionality.
)

(event Collision|EventActorBeginOverlap
  (params (OtherActor :type Actor%20Object%20Reference))
  (|CallParentFunction OtherActor) ; This node is disabled and will not be called.\nDrag off pins to build functionality.
)

(event EventTick
  (params (DeltaSeconds :type Float%20%28single-precision%29))
  (|CallParentFunction DeltaSeconds) ; This node is disabled and will not be called.\nDrag off pins to build functionality.
)

(event EventCETurnOfDestroy
  (|CallParentFunction)
  (Default|StopSequence (Variables|Default|GetCinematic%20Manager)))

(fn ConstructionScript
  (|CallParentFunction))