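; BP_WidgetE is an actor whose widget component turns to face the player while active.
; It starts hidden, with a looping timer paused at BeginPlay.
; SetActive toggles widget visibility and pauses or resumes that timer, which calls UpdateRot to rotate the whole actor toward the player character's location instead of updating on Tick.
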(event Custom|SetActive
  (params (IsActive :type Boolean))
  (bind _timer (Variables|Default|GetTimer))
  (bind _output_get (Variables|Default|SetIsActive IsActive))
  (Rendering|SetVisibility (Variables|Default|GetWidget) _output_get false)
  (if _output_get
    (Utilities|Time|UnpauseTimerbyHandle _timer)
    (else
      (Utilities|Time|PauseTimerbyHandle _timer))))

(event EventBeginPlay
  (bind _returnvalue (Utilities|Time|SetTimerbyFunctionName 0 "UpdateRot" 0.05 true))
  (bind _output_get (Variables|Default|SetTimer _returnvalue))
  (Utilities|Time|PauseTimerbyHandle _output_get)
  (Rendering|SetVisibility (Variables|Default|GetWidget) false false))

(fn ConstructionScript)

(fn UpdateRot
  (Transformation|SetActorRotation (Math|Rotator|FindLookatRotation (Transformation|GetActorLocation) (Transformation|GetActorLocation (Game|GetPlayerCharacter 0)))))