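; Actor component that stores an owner's dialogues and plays them through the in-game HUD.
; PlayDialogue looks up the entry matching an interaction, stamps it with the author name and sends it to the HUD with a voice SFX name.
; It binds to the dialogue widget's finished event, and its DialogueEnd handler unbinds and calls DialogueEnded with the interaction and answer.
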(event Custom|Set%20AuthorName
  (params (AuthorName :type Texture%202D%20Object%20Reference))
  (Variables|Default|SetAuthorName AuthorName))

(event Custom|DialogueEnd
  (params (Dialogue :type ST%20Dialogue%20Structure) (Answer :type Boolean))
  (EventDispatchers|UnbindEventfromFinishedDialogue (Variables|/Game/_projectContent/Widgets/HUD_InGame.HUD_InGame_C|GetWD_Dialogue (Variables|Default|GetHUD)) (delegate Custom|DialogueEnd))
  (Default|CallDialogueEnded (.DialogueInteraction (Utilities|Struct|BreakST_Dialogue Dialogue)) Answer))

(event EventBeginPlay
  (bind _ashud_in_game (Utilities|Casting|CastToHUD_InGame (HUD|GetHUD (Game|GetPlayerController 0)))
    (:then
      (Variables|Default|SetHUD _ashud_in_game))
    (:CastFailed
      (Development|PrintString "Cast Failed"))))

(fn FindDialogue
  (params (Interaction :type EN_DialogueInteraction%20Enum :default "NewEnumerator0"))
  (bind _array_element (Utilities|Array|ForEachLoopwithBreak (Variables|Default|GetDialogues))
    (:LoopBody
      (if (Utilities|Enum|Equal(Enum) Interaction (.DialogueInteraction (Utilities|Struct|BreakST_Dialogue _array_element)))
        (return true (Utilities|Struct|MakeST_Dialogue (.DialogueInteraction (Utilities|Struct|BreakST_Dialogue _array_element)) (Variables|Default|GetAuthorName) (.Content (Utilities|Struct|BreakST_Dialogue _array_element)) (.IsQuestion (Utilities|Struct|BreakST_Dialogue _array_element)) (.PositiveAnswer (Utilities|Struct|BreakST_Dialogue _array_element)) (.NegativeAnswer (Utilities|Struct|BreakST_Dialogue _array_element))))))
    (:Completed
      (return false ""))))

(fn PlayDialogue
  (params (Interaction :type EN_DialogueInteraction%20Enum :default "NewEnumerator0"))
  (bind _hud (Variables|Default|GetHUD))
  (bind (_dialogueexist _dialogue) (CallFunction|FindDialogue Interaction))
  (if _dialogueexist
    (Default|DisplayDialogue _hud _dialogue (Variables|Default|GetSFXVoice%20Name))
    (EventDispatchers|BindEventtoFinishedDialogue (Variables|/Game/_projectContent/Widgets/HUD_InGame.HUD_InGame_C|GetWD_Dialogue _hud) (EventDispatchers|CreateEvent :!event Custom|DialogueEnd))
    (else
      (Development|PrintString "No Dialogue Setup"))))