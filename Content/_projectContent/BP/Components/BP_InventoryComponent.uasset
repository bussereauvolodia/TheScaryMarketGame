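; BP_InventoryComponent is an inventory component that stores items in an Inventory array and exposes functions to read and edit it.
; AddItem appends without a capacity check, and RemoveItem removes an item only if present.
; IsInventoryFull returns true while the length is at or below InventoryMaxLength, the reverse of its name.
; GetItemAtIndex always reads at InventoryMaxLength, and ClearItem only copies Inventory into InventoryCopy without emptying it.
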(fn IsInventoryFull
  (return (>= (Variables|Default|GetInventoryMaxLength) (Utilities|Array|Length (Variables|Default|GetInventory)))))

(fn GetInventory
  (return (Variables|Default|GetInventory)))

(fn AddItem
  (params (Item :type ST%20Item%20Informations%20Structure))
  (Utilities|Array|Add (Variables|Default|GetInventory) Item)
  (return))

(fn GetItematIndex
  (return (Utilities|Array|Get(acopy) (Variables|Default|GetInventory) (Variables|Default|GetInventoryMaxLength))))

(fn ClearItem
  (LocalVariables|SetInventoryCopy (Variables|Default|GetInventory)))

(fn RemoveItem
  (params (Item :type ST%20Item%20Informations%20Structure))
  (bind _inventory (Variables|Default|GetInventory))
  (if (Utilities|Array|ContainsItem _inventory Item)
    (Utilities|Array|RemoveItem _inventory Item)))