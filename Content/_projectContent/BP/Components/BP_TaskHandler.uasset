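; BP_TaskHandler is a task component that tracks required items and lets them be paid in from an inventory.
; CompleteTask finds the first required item the inventory contains, lowers its remaining count, removes the items and calls TaskChanged.
; It returns after that single match with the task's GameplayElements and a completion flag from IsTaskComplete, which checks that no required count remains above zero.
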(fn GetTask
  (return (Variables|Default|GetTask)))

(fn CompleteTask
  (params (Inventory :type BP%20Inventory%20Component%20Object%20Reference))
  (bind _task (Variables|Default|GetTask))
  (for (_array_element _array_index) (.requireditems _task)
    (bind _result (Default|ContainsItem Inventory (.requireditem _array_element)))
    (if _result
      (bind _count (Default|GetItemCount Inventory (.requireditem _array_element)))
      (Utilities|Array|SetArrayElem (.requireditems _task) _array_index (Utilities|Struct|MakeST_RequiredItem (.requireditem _array_element) (- (.requiredcount _array_element) _count)))
      (Default|RemoveItems Inventory (.requireditem _array_element) (Math|Integer|Clamp(Integer) (.requiredcount _array_element) 0 _count))
      (bind _isfinished (CallFunction|IsTaskComplete))
      (Default|CallTaskChanged)
      (return _isfinished (.gameplayelements (Variables|Default|GetTask))))))

(fn IsTaskComplete
  (bind _array_element (Utilities|Array|ForEachLoopwithBreak (.requireditems (Variables|Default|GetTask)) :!label _label)
    (:LoopBody
      (if (> (.requiredcount _array_element) 0)
        (LocalVariables|SetIsUnfinished true)
        (goto _label Break)))
    (:Completed
      (return (not (LocalVariables|GetIsUnfinished))))))