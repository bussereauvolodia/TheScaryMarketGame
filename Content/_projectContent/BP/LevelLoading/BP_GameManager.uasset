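; Game manager that streams in the game's zones as the player progresses, starting with the safe zone on BeginPlay.
; A shared LoadLevel event does a blocking stream load, makes the level visible and can notify a listening actor when finished.
; OnTaskCollected loads the main zone for one gameplay element type and, independently, the second or third zone based on the task's key index.
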(event Custom|LoadLevel
  (params (LevelName :type Name) (HasListenningActor :type Boolean) (ListenningActor :type IN%20Level%20Loading%20Sensible%20Interface))
  (Game|LoadStreamLevel(byName) LevelName true true)
  (if HasListenningActor
    (Default|LevelFinishedLoad ListenningActor)))

(event Custom|OnTaskCollected
  (params (Task :type ST%20Task%20Structure))
  (Utilities|FlowControl|Sequence
    (:then_0
      (if (Utilities|Enum|Equal(Enum) (.gameplayelements Task) "NewEnumerator4")
        (CallFunction|LoadLevel (Variables|Default|GetMainZone) false)))
    (:then_1
      (switch int (.keyindex Task)
        (:0
          (CallFunction|LoadLevel (Variables|Default|Get2ndZone) false))
        (:1
          (CallFunction|LoadLevel (Variables|Default|Get3rdZone) false))))))

(event EventBeginPlay
  (CallFunction|LoadLevel (Variables|Default|GetSafeZoneLevel) false))

(fn ConstructionScript)