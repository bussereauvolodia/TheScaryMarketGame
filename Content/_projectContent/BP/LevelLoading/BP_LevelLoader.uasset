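; BP_LevelLoader is a trigger actor that requests a streaming level load through BP_GameManager when the player character enters its Zone.
; It caches the game manager on BeginPlay.
; On overlap, if IsUnloading is false and the IsLoadedMessage check on the named streaming level returns true, it calls the manager's LoadLevel with no listening actor.
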(event OnComponentBeginOverlap(Zone)
  (params (OverlappedComponent :type Primitive%20Component%20Object%20Reference) (OtherActor :type Actor%20Object%20Reference) (OtherComp :type Primitive%20Component%20Object%20Reference) (OtherBodyIndex :type Integer) (bFromSweep :type Boolean) (SweepResult :type Hit%20Result%20Structure%20%28by%20ref%29))
  (bind _level_name (Variables|Default|GetLevel%20Name))
  (if (== OtherActor (Game|GetPlayerCharacter 0))
    (if (not (Variables|Default|GetIsUnloading))
      (bind _returnvalue (Class|LevelInstanceInterface|IsLoaded(Message) (Class|GameplayStatics|GetStreamingLevel _level_name)))
      (if _returnvalue
        (Default|LoadLevel (Variables|Default|GetGameManager) _level_name false)))))

(event EventBeginPlay
  (bind _returnvalue (Actor|GetActorOfClass "/Game/_projectContent/BP/LevelLoading/BP_GameManager.BP_GameManager_C"))
  (Variables|Default|SetGameManager _returnvalue))

(fn ConstructionScript)