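; BP_AudioManager manages background music, switching between a level track and a safe-zone hub track.
; On BeginPlay it looks up both BGM rows in DT_SoundInfos, spawns a random sound from each as 2D audio, and stores the components, stopping neither.
; ChangedZone takes a safe-zone flag, plays the matching component from the start and stops the other, with validity checks and no crossfade.
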(event Custom|ChangedZone
  (params (IsInSafeZone :type Boolean))
  (bind _safezonemussound (Variables|Default|GetSafeZoneMusSound))
  (bind _levelmussound (Variables|Default|GetLevelMusSound))
  (if IsInSafeZone
    (Utilities|IsValid _safezonemussound
      (:Is%20Valid
        (Audio|Components|Audio|Play _safezonemussound 0.0))
      (:Is%20Not%20Valid
        _))
    (Utilities|IsValid _levelmussound
      (:Is%20Valid
        (Audio|Components|Audio|Stop _levelmussound)))
    (else
      (Utilities|IsValid _safezonemussound
        (:Is%20Valid
          (Audio|Components|Audio|Stop _safezonemussound))
        (:Is%20Not%20Valid
          _))
      (Utilities|IsValid _levelmussound
        (:Is%20Valid
          (Audio|Components|Audio|Play _levelmussound 0.0))))))

(event EventBeginPlay
  (bind _returnvalue (Utilities|GetDataTableRow "/Game/_projectContent/DataTables/DT_SoundInfos.DT_SoundInfos" "BGMLevel")
    (:then
      (bind _returnvalue_2 (Audio|SpawnSound2D (.OutItem (Utilities|Array|Random (.sfxfile _returnvalue))) 1.0 1.0 0.0 0 false false))
      (Variables|Default|SetLevelMusSound _returnvalue_2)
      (bind _returnvalue_3 (Utilities|GetDataTableRow "/Game/_projectContent/DataTables/DT_SoundInfos.DT_SoundInfos" "BGMHubGlobal")
        (:then
          (bind _returnvalue_4 (Audio|SpawnSound2D (.OutItem (Utilities|Array|Random (.sfxfile _returnvalue_3))) 1.0 1.0 0.0 0 false false))
          (Variables|Default|SetSafeZoneMusSound _returnvalue_4))))))

(fn ConstructionScript)