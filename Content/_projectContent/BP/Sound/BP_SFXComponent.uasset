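; SFX component that plays sounds by name, picking a random variant from the matching DT_SoundInfos row.
; Spatialized plays apply row volume and concurrency, report AI noise for flagged rows, and track audio components for stopping; a separate function plays untracked 2D sounds.
; Stopping works globally or by name, though fade-in plays skip the name list.
; Fade-out calls Stop immediately after FadeOut, and an auto-generated function prunes finished sounds.
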(fn PlaySFX
  (params (SFXName :type String) (Location :type Vector) (Multiplier :type Float%20%28double-precision%29) (Instigator :type Actor%20Object%20Reference))
  (bind _returnvalue (Utilities|GetDataTableRow "/Game/_projectContent/DataTables/DT_SoundInfos.DT_SoundInfos" (Utilities|String|StringToName SFXName))
    (:then
      (bind _output_get (LocalVariables|SetRandomSound (.OutItem (Utilities|Array|Random (.sfxfile _returnvalue)))))
      (bind _returnvalue_2 (Audio|SpawnSoundatLocation _output_get Location "0, 0, 0" (* Multiplier (.intensity _returnvalue)) 1.0 0.0 0 (.concurrencysettings _returnvalue) (.autodestroy _returnvalue)))
      (Utilities|Array|Add (Variables|Default|GetSounds) _returnvalue_2)
      (EventDispatchers|BindEventtoOnAudioFinished _returnvalue_2 (EventDispatchers|CreateEvent :!event BPSFXComponentAutoGenFunc))
      (Utilities|Array|Add (Variables|Default|GetSoundsPlayed) (Utilities|Struct|MakeST_SoundPlayed SFXName _returnvalue_2))
      (if (.isiasensible _returnvalue)
        (Class|AISenseHearing|ReportNoiseEvent Location (* Multiplier (.intensity _returnvalue)) Instigator (.maxrange _returnvalue) (.sfxtag _returnvalue))
        (return (Variables|/Script/Engine.SoundBase|GetDuration _output_get))
        (else
          (return (Variables|/Script/Engine.SoundBase|GetDuration _output_get)))))
    (:RowNotFound
      (Development|PrintString (Utilities|String|Append "Sound : \"" SFXName "\" Does not exist")))))

(fn PlayNonSpacializedSFX
  (params (SFXName :type String))
  (bind _returnvalue (Utilities|GetDataTableRow "/Game/_projectContent/DataTables/DT_SoundInfos.DT_SoundInfos" (Utilities|String|StringToName SFXName))
    (:then
      (Audio|PlaySound2D (.OutItem (Utilities|Array|Random (.sfxfile _returnvalue))) 1.0 1.0 0.0 0 0))))

(fn StopSFX
  (for _array_element (Variables|Default|GetSounds)
    (Utilities|IsValid _array_element
      (:Is%20Valid
        (Audio|Components|Audio|Stop _array_element))))
  (Utilities|Array|Clear (Variables|Default|GetSounds))
  (return))

(fn PlaySFXwithFade
  (params (SFXName :type String) (Location :type Vector) (Multiplier :type Float%20%28double-precision%29) (Instigator :type Actor%20Object%20Reference) (FadeInDuration :type Float%20%28single-precision%29))
  (bind _returnvalue (Utilities|GetDataTableRow "/Game/_projectContent/DataTables/DT_SoundInfos.DT_SoundInfos" (Utilities|String|StringToName SFXName))
    (:then
      (bind _output_get (LocalVariables|SetRandomSound (.OutItem (Utilities|Array|Random (.sfxfile _returnvalue)))))
      (bind _returnvalue_2 (Audio|SpawnSoundatLocation _output_get Location "0, 0, 0" (* Multiplier (.intensity _returnvalue)) 1.0 0.0 0 (.concurrencysettings _returnvalue) (.autodestroy _returnvalue)))
      (Utilities|Array|Add (Variables|Default|GetSounds) _returnvalue_2)
      (Audio|Components|Audio|FadeIn _returnvalue_2 FadeInDuration 1.0 0.0 "Linear" :!class /Script/Engine.AudioComponent)
      (if (.isiasensible _returnvalue)
        (Class|AISenseHearing|ReportNoiseEvent Location (* Multiplier (.intensity _returnvalue)) Instigator (.maxrange _returnvalue) (.sfxtag _returnvalue))
        (return (Variables|/Script/Engine.SoundBase|GetDuration _output_get))))
    (:RowNotFound
      (Development|PrintString (Utilities|String|Append "Sound : \"" SFXName "\" Does not exist")))))

(fn StopSFXwithFade
  (params (FadeOutDuration :type Float%20%28single-precision%29))
  (for _array_element (Variables|Default|GetSounds)
    (Utilities|IsValid _array_element
      (:Is%20Valid
        (Audio|Components|Audio|FadeOut _array_element FadeOutDuration 0.0 "Linear" :!class /Script/Engine.AudioComponent)
        (Audio|Components|Audio|Stop _array_element))))
  (Utilities|Array|Clear (Variables|Default|GetSounds))
  (return))

(fn StopSFXfromName
  (params (Name :type String))
  (for _array_element (Variables|Default|GetSoundsPlayed)
    (if (Utilities|Enum|Equal(Enum) Name (.sfxname _array_element))
      (Audio|Components|Audio|Stop (.sound _array_element)))))

(fn BPSFXComponentAutoGenFunc
  (bind _sounds (Variables|Default|GetSounds))
  (for _array_element _sounds
    (if (not (Audio|Components|Audio|IsPlaying _array_element))
      (Utilities|Array|RemoveItem _sounds _array_element)))
  (Development|PrintString (Utilities|String|ToString(Integer) (Utilities|Array|Length _sounds))))